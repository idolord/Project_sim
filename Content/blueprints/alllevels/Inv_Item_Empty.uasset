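; Inv_Item_Empty is an inventory item Blueprint that, by its name, represents an empty item or slot.
; It provides the inventory item query functions with null-object style results.
; Stack, spawn, extract, use and refine checks all return false, remaining stack amount returns zero, and the info and actor getters return no values.
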(fn GetInvInfo
  (return ""))

(fn GetInvItemInfo
  (return ""))

(fn GetInvItemCanStack?
  (return false))

(fn GetInvItemCanSpawn?
  (return false))

(fn GetInvItemCanExtract?
  (return false))

(fn GetInvItemCanUse?
  (return false))

(fn GetInvItemIsRefinable?
  (return false))

(fn GetInvItemActor
  (return 0))

(fn GetInvItemStackAmountLeft
  (return 0.0))
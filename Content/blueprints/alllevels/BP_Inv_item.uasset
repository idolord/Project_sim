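; BP_Inv_item represents an inventory item, identified by a RowName into the Items data table and carrying its own ItemAmount.
; Getter functions look up that row for item info, stack, spawn, extract, use and refine flags, world actor and stack limit, printing an error if it is missing.
; Remaining stack space is the row's limit minus ItemAmount.
; The use and drop functions are empty stubs.
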(fn GetInvInfo
  (bind _row_name (Variables|Default|Getrow_name))
  (bind _returnvalue (Utilities|GetDataTableRow "/Game/blueprints/alllevels/data/items.items" _row_name)
    (:then
      (return _returnvalue))
    (:RowNotFound
      (Development|PrintString 0 (Utilities|String|Append "Object: " (Utilities|String|ToString(Name) _row_name) "does not exist!"))
      (return ""))))

(fn GetInvItemInfo
  (bind _row_name (Variables|Default|Getrow_name))
  (bind _returnvalue (Utilities|GetDataTableRow "/Game/blueprints/alllevels/data/items.items" _row_name)
    (:then
      (return (.ItemInfo (Utilities|Struct|BreakItem_Inv_Info _returnvalue))))
    (:RowNotFound
      (Development|PrintString 0 (Utilities|String|Append "Object: " (Utilities|String|ToString(Name) _row_name) "does not exist!"))
      (return ""))))

(fn GetInvItemCanStack?
  (bind _row_name (Variables|Default|Getrow_name))
  (bind _returnvalue (Utilities|GetDataTableRow "/Game/blueprints/alllevels/data/items.items" _row_name)
    (:then
      (return (.CanStack? (Utilities|Struct|BreakItem_Inv_Info _returnvalue))))
    (:RowNotFound
      (Development|PrintString 0 (Utilities|String|Append "Object: " (Utilities|String|ToString(Name) _row_name) "does not exist!"))
      (return false))))

(fn GetInvItemCanSpawn?
  (bind _row_name (Variables|Default|Getrow_name))
  (bind _returnvalue (Utilities|GetDataTableRow "/Game/blueprints/alllevels/data/items.items" _row_name)
    (:then
      (return (.CanSpawn? (Utilities|Struct|BreakItem_Inv_Info _returnvalue))))
    (:RowNotFound
      (Development|PrintString 0 (Utilities|String|Append "Object: " (Utilities|String|ToString(Name) _row_name) "does not exist!"))
      (return false))))

(fn GetInvItemCanExtract?
  (bind _row_name (Variables|Default|Getrow_name))
  (bind _returnvalue (Utilities|GetDataTableRow "/Game/blueprints/alllevels/data/items.items" _row_name)
    (:then
      (return (.CanExtract? (Utilities|Struct|BreakItem_Inv_Info _returnvalue))))
    (:RowNotFound
      (Development|PrintString 0 (Utilities|String|Append "Object: " (Utilities|String|ToString(Name) _row_name) "does not exist!"))
      (return false))))

(fn GetInvItemCanUse?
  (bind _row_name (Variables|Default|Getrow_name))
  (bind _returnvalue (Utilities|GetDataTableRow "/Game/blueprints/alllevels/data/items.items" _row_name)
    (:then
      (return (.CanUse? (Utilities|Struct|BreakItem_Inv_Info _returnvalue))))
    (:RowNotFound
      (Development|PrintString 0 (Utilities|String|Append "Object: " (Utilities|String|ToString(Name) _row_name) "does not exist!"))
      (return false))))

(fn GetInvItemIsRefinable?
  (bind _row_name (Variables|Default|Getrow_name))
  (bind _returnvalue (Utilities|GetDataTableRow "/Game/blueprints/alllevels/data/items.items" _row_name)
    (:then
      (return (.IsRefinable? (Utilities|Struct|BreakItem_Inv_Info _returnvalue))))
    (:RowNotFound
      (Development|PrintString 0 (Utilities|String|Append "Object: " (Utilities|String|ToString(Name) _row_name) "does not exist!"))
      (return false))))

(fn GetInvItemActor
  (bind _row_name (Variables|Default|Getrow_name))
  (bind _returnvalue (Utilities|GetDataTableRow "/Game/blueprints/alllevels/data/items.items" _row_name)
    (:then
      (return (.WorldActor (Utilities|Struct|BreakItem_Inv_Info _returnvalue))))
    (:RowNotFound
      (Development|PrintString 0 (Utilities|String|Append "Object: " (Utilities|String|ToString(Name) _row_name) "does not exist!"))
      (return 0))))

(fn OnUse)

(fn OnDrop)

(fn GetInvItemStackAmountLeft
  (bind _row_name (Variables|Default|Getrow_name))
  (bind _returnvalue (Utilities|GetDataTableRow "/Game/blueprints/alllevels/data/items.items" _row_name)
    (:then
      (return (- (.StaskLimit (Utilities|Struct|BreakItem_Inv_Info _returnvalue)) (Variables|Default|Getitem_amount))))
    (:RowNotFound
      (Development|PrintString 0 (Utilities|String|Append "Object: " (Utilities|String|ToString(Name) _row_name) "does not exist!"))
      (return -1.0))))

(fn GetInvItemAmount
  (return (Variables|Default|Getitem_amount)))

(fn SetInvItemAmount
  (params (item_amount :type Float%20%28single-precision%29))
  (Variables|Default|Setitem_amount item_amount))

(fn GetInvItemMaxStackAmount
  (bind _row_name (Variables|Default|Getrow_name))
  (bind _returnvalue (Utilities|GetDataTableRow "/Game/blueprints/alllevels/data/items.items" _row_name)
    (:then
      (return (.StaskLimit (Utilities|Struct|BreakItem_Inv_Info _returnvalue))))
    (:RowNotFound
      (Development|PrintString 0 (Utilities|String|Append "Object: " (Utilities|String|ToString(Name) _row_name) "does not exist!"))
      (return -1.0))))
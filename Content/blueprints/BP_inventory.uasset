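; Slot-based inventory Blueprint that stores stackable items as an array of item objects, filled with Inv_Item_Empty placeholders on BeginPlay.
; AddItem requires an empty slot, tops up a stack of the same class and puts overflow in an empty slot.
; It has no branch for placing an item class not already held.
; RemoveItem reduces or empties matching stacks, reporting success and amount removed.
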(event EventBeginPlay
  (CallFunction|InitInventory))

(fn GetInventory
  (return (Variables|Default|Getinventory)))

(fn InitInventory
  (Utilities|Array|Clear (Variables|Default|Getinventory))
  (for _index (range 0 (- (Variables|Default|GetInv_Slots) 1))
    (bind _returnvalue (Game|ConstructObjectfromClass "/Game/blueprints/items/inv/Inv_Item_Empty.Inv_Item_Empty_C" self))
    (Utilities|Array|Add (Variables|Default|Getinventory) _returnvalue)))

(fn AddItem
  (params (item_to_add :type BP%20Inv%20Item%20Class%20Reference) (amt_to_add :type Float%20%28single-precision%29))
  (bind (_has_slot_ _openslots) (CallFunction|HasSlotinInv))
  ;[1 1 1] getting imput
  (LocalVariables|SetLocalItem item_to_add)
  (LocalVariables|SetLocalAmt amt_to_add)
  ;[1 1 1] if inv has slot available get how many else fail
  (if _has_slot_
    (LocalVariables|SetLocal_open_spaces _openslots)
    ;[1 1 1] Comment
    (for _array_element (Variables|Default|Getinventory)
      (if (== (Utilities|GetClass _array_element) (LocalVariables|GetLocalItem))
        (LocalVariables|SetLocal_Item _array_element)
        ;[1 1 1] check in item can stack
        (if true
          ;[1 1 1] if stack isn't full
          (if (> (Default|GetInvItemStackAmountLeft (LocalVariables|GetLocal_Item)) 0.0)
            ;[1 1 1] comparing for remaining space
            (if (<= (+ (Default|GetInvItemAmount (LocalVariables|GetLocal_Item)) (LocalVariables|GetLocalAmt)) (Default|GetInvItemMaxStackAmount (LocalVariables|GetLocal_Item)))
              ;[1 1 1] adding to inventory
              (Default|SetInvItemAmount (LocalVariables|GetLocal_Item) (+ (Default|GetInvItemAmount (LocalVariables|GetLocal_Item)) (LocalVariables|GetLocalAmt)))
              (return true)
              (else
                ;[1 1 1] if we have other slots to check continue otherwise fail
                (if (> (LocalVariables|GetLocal_open_spaces) 0)
                  ;[1 1 1] adding
                  (LocalVariables|SetLocalAmt (- (LocalVariables|GetLocalAmt) (Default|GetInvItemStackAmountLeft (LocalVariables|GetLocal_Item))))
                  (Default|SetInvItemAmount (LocalVariables|GetLocal_Item) (Default|GetInvItemMaxStackAmount (LocalVariables|GetLocal_Item)))
                  ;[1 1 1] loop for empty slot to put in
                  (bind (_array_element_2 _array_index) (Utilities|Array|ForEachLoopwithBreak (Variables|Default|Getinventory) :!label _label)
                    (:LoopBody
                      (if (== (Utilities|GetClass _array_element_2) "/Game/blueprints/items/inv/Inv_Item_Empty.Inv_Item_Empty_C")
                        (LocalVariables|SetLocal%20index _array_index)
                        (goto _label Break)
                        (else
                          (LocalVariables|SetLocal%20index -1))))
                    (:Completed
                      (if (>= (LocalVariables|GetLocal%20index) 0)
                        (bind _returnvalue (Game|ConstructObjectfromClass (LocalVariables|GetLocalItem) self))
                        (Default|SetInvItemAmount _returnvalue (LocalVariables|GetLocalAmt))
                        (Utilities|Array|SetArrayElem (Variables|Default|Getinventory) (LocalVariables|GetLocal%20index) _returnvalue)
                        (return true)
                        (else
                          (return false)))))
                  (else
                    (return false))))))
          (else
            (goto _label)))
        (else
          (goto _label))))
    (else
      (return false))))

(fn HasSlotinInv
  (bind _local_open_slots (LocalVariables|GetLocal_open_slots))
  (for _array_element (Variables|Default|Getinventory)
    (if (== (Utilities|GetClass _array_element) "/Game/blueprints/items/inv/Inv_Item_Empty.Inv_Item_Empty_C")
      (Math|Integer|IncrementInt (LocalVariables|GetLocal_open_slots))))
  (return (> _local_open_slots 0) _local_open_slots))

(fn RemoveItem
  (params (item_to_remove :type BP%20Inv%20Item%20Class%20Reference) (amt_to_remove :type Float%20%28single-precision%29))
  ;[1 1 1] getting imput
  (LocalVariables|SetLocalItem item_to_remove)
  (LocalVariables|SetLocalAmt amt_to_remove)
  (LocalVariables|Setlocal_required_amt amt_to_remove)
  ;[1 1 1] Comment
  (for (_array_element _array_index) (Variables|Default|Getinventory)
    (if (== (Utilities|GetClass _array_element) (LocalVariables|GetLocalItem))
      (LocalVariables|SetLocal_Item _array_element)
      ;[1 1 1] check in item can stack
      (if true
        ;[1 1 1] comparing for available ammount
        (if (> (- (Default|GetInvItemAmount (LocalVariables|GetLocal_Item)) (LocalVariables|GetLocalAmt)) 0.0)
          ;[1 1 1] removing from inventory
          (Default|SetInvItemAmount (LocalVariables|GetLocal_Item) (- (Default|GetInvItemAmount (LocalVariables|GetLocal_Item)) (LocalVariables|GetLocalAmt)))
          (return true (LocalVariables|GetLocalAmt))
          (else
            ;[1 1 1] removing
            (LocalVariables|Setlocal_retrived_amt (LocalVariables|GetLocalAmt))
            (LocalVariables|SetLocalAmt (- (LocalVariables|GetLocalAmt) (Default|GetInvItemStackAmountLeft (LocalVariables|GetLocal_Item))))
            (bind _returnvalue (Game|ConstructObjectfromClass "/Game/blueprints/items/inv/Inv_Item_Empty.Inv_Item_Empty_C" self))
            (Utilities|Array|SetArrayElem (Variables|Default|Getinventory) _array_index _returnvalue)))))
    ;[1 1 1] loop for more slots to remove from
    (bind (_array_element_2 _array_index_2) (Utilities|Array|ForEachLoopwithBreak (Variables|Default|Getinventory) :!label _label)
      (:LoopBody
        (if (== (Utilities|GetClass _array_element_2) (LocalVariables|GetLocalItem))
          (bind _output_get (LocalVariables|SetLocal%20index _array_index_2))
          (bind _output_get_2 (LocalVariables|SetLocalAmt (- (LocalVariables|GetLocalAmt) (Default|GetInvItemStackAmountLeft (Utilities|Array|Get(acopy) (Variables|Default|Getinventory) _output_get)))))
          (LocalVariables|Setlocal_retrived_amt (+ (LocalVariables|Getlocal_retrived_amt) (- (LocalVariables|GetLocalAmt) (Default|GetInvItemStackAmountLeft (Utilities|Array|Get(acopy) (Variables|Default|Getinventory) _output_get)))))
          (if (> _output_get_2 0.0)
            (bind _returnvalue_2 (Game|ConstructObjectfromClass "/Game/blueprints/items/inv/Inv_Item_Empty.Inv_Item_Empty_C" self))
            (Utilities|Array|SetArrayElem (Variables|Default|Getinventory) _output_get _returnvalue_2)
            (else
              (Utilities|FlowControl|Sequence
                (:then_0
                  (Default|SetInvItemAmount (Utilities|Array|Get(acopy) (Variables|Default|Getinventory) _output_get) (- (Default|GetInvItemAmount (Utilities|Array|Get(acopy) (Variables|Default|Getinventory) _output_get)) (LocalVariables|GetLocalAmt)))
                  (LocalVariables|Setlocal_retrived_amt (+ (- (Default|GetInvItemAmount (Utilities|Array|Get(acopy) (Variables|Default|Getinventory) _output_get)) (LocalVariables|GetLocalAmt)) (LocalVariables|Getlocal_retrived_amt))))
                (:then_1
                  (goto _label Break)))))
          (else
            (LocalVariables|SetLocal%20index -1))))
      (:Completed
        (if (< (LocalVariables|Getlocal_retrived_amt) (LocalVariables|Getlocal_required_amt))
          (return false (LocalVariables|Getlocal_retrived_amt))
          (else
            (return true (LocalVariables|Getlocal_required_amt))))))))
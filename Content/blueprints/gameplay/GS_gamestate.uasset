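; GS_gamestate is a game state Blueprint that keeps a list of mainframes and relays idle updates for them.
; anounce_mainframe, noted as called on base_simulationnaute, adds each mainframe to CurrMf.
; update_idle runs an authority-only loop that calls do_update_iddle for every stored mainframe, with debug prints along the way.
; do_update_iddle is an empty stub, and its mainframe name print is disconnected.
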(event Custom|anounce_mainframe
  (params (mainframe :type Mainframe%20Object%20Reference))
  ;[1 1 1] getting mainfraims (called on base_simulationnaute
  (Utilities|Array|Add (Variables|Default|Getcurr_mf) mainframe))

(event Custom|do_update_iddle
  (params (mainframe :type Mainframe%20Object%20Reference)))

(event Custom|update_idle
  (Development|PrintString "Hello")
  (Networking|SwitchHasAuthority
    (:Authority
      (Development|PrintString "paté")
      (for _array_element (Variables|Default|Getcurr_mf)
        (CallFunction|DoUpdateIddle _array_element))
      (Development|PrintString "broadcasted" true true "(R=0.000000,G=0.660000,B=1.000000,A=1.000000)" 15.0))))

(event EventBeginPlay)

(event EventTick
  (params (DeltaSeconds :type Float%20%28single-precision%29)))

(fn ConstructionScript)
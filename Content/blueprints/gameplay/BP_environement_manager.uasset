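; Environment manager that runs the space station's day/night cycle, with elapsed time advanced on the server.
; BeginPlay finds the sky, directional light, clock HUD, mainframe and station mesh, creates a dynamic hull material, and has the authority load saved day/night colors and date.
; Each authority tick updates time, then calls update events that rotate the clock, refresh the sun direction and fade light intensity and the material's timescaler around night hours.
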(event Custom|Update_save_info
  (params (world_sky :type BP%20Sky%20Sphere%20Object%20Reference) (world_light :type Directional%20Light%20Object%20Reference) (world_station_clock%20hud :type Fbx%20Scene%20Station%20Clock%20Hud%20Object%20Reference) (world_mainframe :type Mainframe%20Object%20Reference) (world%20station%20mat :type Material%20Instance%20Dynamic%20Object%20Reference))
  ;[1 1 1] server init
  (Utilities|FlowControl|Sequence
    (:then_0
      (Variables|Day_Cicle|Setsky world_sky))
    (:then_1
      (Variables|Day_Cicle|Setlight world_light))
    (:then_2
      (Variables|Day_Cicle|SetstationClockHud world_station_clock%20hud))
    (:then_3
      (bind _output_get (Variables|Day_Cicle|Setstation world_mainframe)))
    (:then_4
      (Variables|Day_Cicle|Setstation_mat world%20station%20mat))
    (:then_5
      (Utilities|FlowControl|Sequence
        (:then_0
          (Variables|Default|SetDay_Color (.station_color (Utilities|Struct|Breakplayer_info (Variables|/Game/Mainframe/mainframe.mainframe_C|Getplayer_save _output_get)))))
        (:then_1
          (Variables|Default|SetNight_Color (.station_color_night (Utilities|Struct|Breakplayer_info (Variables|/Game/Mainframe/mainframe.mainframe_C|Getplayer_save _output_get)))))
        (:then_2
          (Variables|Default|SetDay_EM_Color (.station_EM_color (Utilities|Struct|Breakplayer_info (Variables|/Game/Mainframe/mainframe.mainframe_C|Getplayer_save _output_get)))))
        (:then_3
          (Variables|Default|SetNight_EM_Color (.station_EM_color_night (Utilities|Struct|Breakplayer_info (Variables|/Game/Mainframe/mainframe.mainframe_C|Getplayer_save _output_get)))))
        (:then_4
          (Variables|Time|Setcurrent_time (.date (Utilities|Struct|Breakplayer_info (Variables|/Game/Mainframe/mainframe.mainframe_C|Getplayer_save _output_get)))))
        (:then_5
          (CallFunction|SetElapsedTimeBasedOfStart))
        (:then_6
          (CallFunction|ServerInitCallback))))))

(event Custom|server_init_callback
  ;[1 1 1] server ask client to set station dinamic material
  (CallFunction|SetDinamicMat self))

(event Custom|OnUpdateHud
  ;[1 1 1] clients updates
  (CallFunction|UpdateSunPos)
  (CallFunction|FadeLights))

(event Custom|Updateserver_time
  ;[1 1 1] server tick:  update time and call clients updates
  (CallFunction|UpdateElapsedTime)
  (CallFunction|UpdateCurrentTime)
  (CallFunction|OnUpdateHud))

(event EventTick
  (params (DeltaSeconds :type Float%20%28single-precision%29))
  ;[1 1 1] haut client: trigger server tick
  (Networking|SwitchHasAuthority
    (:Authority
      (CallFunction|UpdateserverTime))))

(event EventBeginPlay
  ;[1 1 1] clients init
  (Utilities|FlowControl|Sequence
    (:then_0
      (CallFunction|GetClockLightSky))
    (:then_1
      (CallFunction|SetGetLightsIntensity))
    (:then_2
      (bind _output_get (CallFunction|MakeDinamicMat)))
    (:then_3
      (Networking|SwitchHasAuthority
        (:Authority
          (CallFunction|UpdateSaveInfo (Variables|Day_Cicle|Getsky) (Variables|Day_Cicle|Getlight) (Variables|Day_Cicle|GetstationClockHud) (Variables|Day_Cicle|Getstation) _output_get))))))

(fn ConstructionScript
  (Variables|Time|SetSeconds_per_day (* (Variables|Time|GetMinutes_per_day) 6e+01)))

(fn GetClockLightSky
  (Utilities|FlowControl|Sequence
    (:then_0
      (Utilities|IsValid (Variables|Day_Cicle|Getsky)
        (:Is%20Not%20Valid
          (env|GetSky))))
    (:then_1
      (Utilities|IsValid (Variables|Day_Cicle|Getlight)
        (:Is%20Not%20Valid
          (env|GetLight))))
    (:then_2
      (Utilities|IsValid (Variables|Day_Cicle|GetstationClockHud)
        (:Is%20Not%20Valid
          (env|GetStationClock))))
    (:then_3
      (Utilities|IsValid (Variables|Day_Cicle|Getstation)
        (:Is%20Not%20Valid
          (CallFunction|GetMainFrame))))
    (:then_4
      (Utilities|IsValid (Variables|Day_Cicle|Getstation_mesh)
        (:Is%20Not%20Valid
          (CallFunction|GetStationMech))))))

(fn SetGetLightsIntensity
  (Variables|Day_Cicle|SetLights_Intensity (Variables|/Script/Engine.LightComponentBase|GetIntensity (Variables|/Script/Engine.Light|GetLightComponent (Variables|Day_Cicle|Getlight)))))

(fn SetElapsedTimeBasedOfStart
  (Variables|Time|SetElapsed_time (* (CallFunction|GetTimeinSec (Variables|time|GetStart_Time)) (/ (Variables|Time|GetSeconds_per_day) 8.64e+04))))

(fn GetTimeinSec
  (params (Time%20in :type Time%20Struct%20Structure%20%28by%20ref%29))
  (return (+ (* (.days Time%20in) 86400) (* (.hours Time%20in) 3600) (* (.minutes Time%20in) 60))))

(fn UpdateSunPos
  (Transformation|SetActorRotation (Variables|Day_Cicle|GetstationClockHud) (Math|Rotator|MakeRotator 0.0 0.0 (Math|Float|MapRangeClamped (* (* (CallFunction|GetFractionOfDay) -3.6e+02) -1.0) 0.0 3.6e+02 35.0 325.0)))
  (Default|UpdateSunDirection (Variables|Day_Cicle|Getsky)))

(fn GetFractionOfDay
  (return (Math|Float|%(Float) (/ (Variables|Time|GetElapsed_time) (Variables|Time|GetSeconds_per_day)) 1.0)))

(fn UpdateElapsedTime
  (Variables|Time|SetElapsed_time (+ (Variables|Time|GetElapsed_time) (Utilities|Time|GetWorldDeltaSeconds))))

(fn UpdateCurrentTime
  (Variables|Time|Setcurrent_time (CallFunction|GetCurrentTime)))

(fn GetCurrentTime
  (bind _fraction (CallFunction|GetFractionOfDay))
  (return (Utilities|Struct|MakeTime_Struct (Math|Float|Truncate _fraction) (Math|Float|Truncate (* (Math|Float|%(Float) _fraction 1.0) 24.0)) (Math|Float|Truncate (Math|Float|%(Float) (* _fraction 1.44e+03) 6e+01)))))

(fn GetIsNight
  (bind _current_time (Variables|Time|Getcurrent_time))
  (return (or (< (.hours _current_time) (Variables|Time|GetSH_Lights_up)) (>= (.hours _current_time) (Variables|Time|GetSH_Lights_down)))))

(fn FadeLights
  (bind _returnvalue (Utilities|Time|GetWorldDeltaSeconds))
  (bind _is_night (CallFunction|GetIsNight))
  (bind _seconds_per_day (Variables|Time|GetSeconds_per_day))
  (bind _light (Variables|Day_Cicle|Getlight))
  (bind _lights_intensity (Variables|Day_Cicle|GetLights_Intensity))
  (bind _lights_intensity_2 (Variables|Day_Cicle|GetLights_Intensity))
  (bind _returnvalue_2 (/ 24.0 _seconds_per_day))
  (bind _returnvalue_3 (select _is_night -1.0 1.0))
  (bind _lightcomponent (Variables|/Script/Engine.Light|GetLightComponent _light))
  (bind _returnvalue_4 (* _returnvalue _returnvalue_2 _lights_intensity _returnvalue_3))
  (bind _intensity (Variables|/Script/Engine.LightComponentBase|GetIntensity _lightcomponent))
  (bind _returnvalue_5 (+ _intensity _returnvalue_4))
  (bind _returnvalue_6 (Math|Float|Clamp(Float) _returnvalue_5 0.0 _lights_intensity_2))
  (Rendering|Components|Light|SetIntensity _lightcomponent _returnvalue_6)
  (Rendering|Material|SetScalarParameterValue (Variables|Day_Cicle|Getstation_mat) "timescaler" _returnvalue_6 :!class /Script/Engine.MaterialInstanceDynamic))

(fn GetStationClock
  (bind _outactors (Actor|GetAllActorsOfClass "/Game/Geometry/Meshes/scenes/FbxScene_station_clock_hud.FbxScene_station_clock_hud_C"))
  (Variables|Day_Cicle|SetstationClockHud (Utilities|Array|Get(acopy) _outactors)))

(fn GetSky
  (bind _outactors (Actor|GetAllActorsOfClass "/Engine/EngineSky/BP_Sky_Sphere.BP_Sky_Sphere_C"))
  (Variables|Day_Cicle|Setsky (Utilities|Array|Get(acopy) _outactors)))

(fn GetLight
  (bind _outactors (Actor|GetAllActorsOfClass "/Script/Engine.DirectionalLight"))
  (Variables|Day_Cicle|Setlight (Utilities|Array|Get(acopy) _outactors)))

(fn GetMainFrame
  (bind _outactors (Actor|GetAllActorsOfClass "/Game/Mainframe/mainframe.mainframe_C"))
  (Variables|Day_Cicle|Setstation (Utilities|Array|Get(acopy) _outactors)))

(fn MakeDinamicMat
  (Utilities|IsValid (Variables|Day_Cicle|Getstation_mat)
    (:Is%20Not%20Valid
      (bind _returnvalue (Rendering|Material|CreateDynamicMaterialInstance (Variables|/Game/Geometry/Meshes/scenes/FbxScene_station_int.FbxScene_station_int_C|Getstation_hull (Variables|Day_Cicle|Getstation_mesh)) 0 "/Game/Geometry/mats/station_mat.station_mat" :!class /Script/Engine.PrimitiveComponent))
      (bind _output_get (Variables|Day_Cicle|Setstation_mat _returnvalue))
      (return _output_get))))

(fn SetDinamicMat
  (params (mat :type Material%20Instance%20Dynamic%20Object%20Reference))
  (Utilities|FlowControl|Sequence
    (:then_0
      (Rendering|Material|SetVectorParameterValue mat "color" (Variables|Default|GetDay_Color) :!class /Script/Engine.MaterialInstanceDynamic))
    (:then_1
      (Rendering|Material|SetVectorParameterValue mat "color_night" (Variables|Default|GetNight_Color) :!class /Script/Engine.MaterialInstanceDynamic))
    (:then_2
      (Rendering|Material|SetVectorParameterValue mat "EM_color" (Variables|Default|GetDay_EM_Color) :!class /Script/Engine.MaterialInstanceDynamic))
    (:then_3
      (Rendering|Material|SetVectorParameterValue mat "EM_color_night" (Variables|Default|GetNight_EM_Color) :!class /Script/Engine.MaterialInstanceDynamic))))

(fn GetStationMech
  (bind _outactors (Actor|GetAllActorsOfClass "/Game/Geometry/Meshes/scenes/FbxScene_station_int.FbxScene_station_int_C"))
  (Variables|Day_Cicle|Setstation_mesh (Utilities|Array|Get(acopy) _outactors)))
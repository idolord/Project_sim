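; BP_World_Item is a world pickup that adds an item to the interacting character's inventory.
; Its Interaction event calls AddItem on the character's BPInventory with its ItemToAdd class and amount.
; On success it prints a confirmation and destroys itself through the destroy_self_all event; on failure it prints an error and stays in the world.
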(event Custom|destroy_self_all
  (Actor|DestroyActor))

(event EventInteraction
  (params (Char_ref :type Base%20Simulationaute%20Object%20Reference))
  (bind _item_to_add (Variables|Default|Getitem_to_add))
  (bind _added_item_ (Default|AddItem (Variables|/Game/blueprints/char/base_simulationaute.base_simulationaute_C|GetBP_inventory Char_ref) _item_to_add (Variables|Default|GetAmt_To_add)))
  (if _added_item_
    (Development|PrintString (Utilities|String|Append "item added: " (Utilities|GetClassDisplayName _item_to_add)) true true "(R=0.292471,G=1.000000,B=0.268382,A=1.000000)")
    (CallFunction|DestroySelfAll)
    (else
      (Development|PrintString "item adding failed" true true "(R=1.000000,G=0.208059,B=0.227956,A=1.000000)"))))

(fn ConstructionScript)